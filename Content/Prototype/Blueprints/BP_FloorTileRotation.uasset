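; Turn tile for an endless-runner prototype that lets the RunCharacter rotate and branch in one of four directions.
; Overlapping CanTurnTrigger enables the character's CanRotate.
; Each of the Up, Down, Right and Left end triggers disables it, records the direction in PrototypeGameMode, calls AddFloorTile, then destroys the tile after a short delay.
; GetAttachTransformRotation exposes the four attach-point world transforms.
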(event `self.CanTurnTrigger.OnComponentBeginOverlap`
  (params (OverlappedComponent :type "PrimitiveComponent Object Reference") (OtherActor :type "Actor Object Reference") (OtherComp :type "PrimitiveComponent Object Reference") (OtherBodyIndex :type Integer) (bFromSweep :type Boolean) (SweepResult :type "HitResult Structure (by ref)"))
  (bind _asrun_character (cast `/Game/Prototype/Blueprints/RunCharacter` OtherActor))
  (set `/Game/Prototype/Blueprints/RunCharacter.CanRotate` true _asrun_character))

(event `self.EndTriggerUp.OnComponentBeginOverlap`
  (params (OverlappedComponent :type "PrimitiveComponent Object Reference") (OtherActor :type "Actor Object Reference") (OtherComp :type "PrimitiveComponent Object Reference") (OtherBodyIndex :type Integer) (bFromSweep :type Boolean) (SweepResult :type "HitResult Structure (by ref)"))
  (bind _asrun_character (cast `/Game/Prototype/Blueprints/RunCharacter` OtherActor))
  (set `/Game/Prototype/Blueprints/RunCharacter.CanRotate` false _asrun_character)
  (bind _asprototype_game_mode (cast `/Game/Prototype/Blueprints/PrototypeGameMode` (`GameplayStatics.GetGameMode`)))
  (set `/Game/Prototype/Blueprints/PrototypeGameMode.RotationDoneTo` "NewEnumerator0" _asprototype_game_mode)
  (`/Game/Prototype/Blueprints/PrototypeGameMode.AddFloorTile` _asprototype_game_mode)
  (`KismetSystemLibrary.Delay` 2.0)
  (`self.K2_DestroyActor`))

(event `self.EndTriggerDown.OnComponentBeginOverlap`
  (params (OverlappedComponent :type "PrimitiveComponent Object Reference") (OtherActor :type "Actor Object Reference") (OtherComp :type "PrimitiveComponent Object Reference") (OtherBodyIndex :type Integer) (bFromSweep :type Boolean) (SweepResult :type "HitResult Structure (by ref)"))
  (bind _asrun_character (cast `/Game/Prototype/Blueprints/RunCharacter` OtherActor))
  (set `/Game/Prototype/Blueprints/RunCharacter.CanRotate` false _asrun_character)
  (bind _asprototype_game_mode (cast `/Game/Prototype/Blueprints/PrototypeGameMode` (`GameplayStatics.GetGameMode`)))
  (set `/Game/Prototype/Blueprints/PrototypeGameMode.RotationDoneTo` "NewEnumerator1" _asprototype_game_mode)
  (`/Game/Prototype/Blueprints/PrototypeGameMode.AddFloorTile` _asprototype_game_mode)
  (`KismetSystemLibrary.Delay` 2.0)
  (`self.K2_DestroyActor`))

(event `self.EndTriggerRight.OnComponentBeginOverlap`
  (params (OverlappedComponent :type "PrimitiveComponent Object Reference") (OtherActor :type "Actor Object Reference") (OtherComp :type "PrimitiveComponent Object Reference") (OtherBodyIndex :type Integer) (bFromSweep :type Boolean) (SweepResult :type "HitResult Structure (by ref)"))
  (bind _asrun_character (cast `/Game/Prototype/Blueprints/RunCharacter` OtherActor))
  (set `/Game/Prototype/Blueprints/RunCharacter.CanRotate` false _asrun_character)
  (bind _asprototype_game_mode (cast `/Game/Prototype/Blueprints/PrototypeGameMode` (`GameplayStatics.GetGameMode`)))
  (set `/Game/Prototype/Blueprints/PrototypeGameMode.RotationDoneTo` "NewEnumerator2" _asprototype_game_mode)
  (`/Game/Prototype/Blueprints/PrototypeGameMode.AddFloorTile` _asprototype_game_mode)
  (`KismetSystemLibrary.Delay` 2.0)
  (`self.K2_DestroyActor`))

(event `self.EndTriggerLeft.OnComponentBeginOverlap`
  (params (OverlappedComponent :type "PrimitiveComponent Object Reference") (OtherActor :type "Actor Object Reference") (OtherComp :type "PrimitiveComponent Object Reference") (OtherBodyIndex :type Integer) (bFromSweep :type Boolean) (SweepResult :type "HitResult Structure (by ref)"))
  (bind _asrun_character (cast `/Game/Prototype/Blueprints/RunCharacter` OtherActor))
  (set `/Game/Prototype/Blueprints/RunCharacter.CanRotate` false _asrun_character)
  (bind _asprototype_game_mode (cast `/Game/Prototype/Blueprints/PrototypeGameMode` (`GameplayStatics.GetGameMode`)))
  (set `/Game/Prototype/Blueprints/PrototypeGameMode.RotationDoneTo` "NewEnumerator3" _asprototype_game_mode)
  (`/Game/Prototype/Blueprints/PrototypeGameMode.AddFloorTile` _asprototype_game_mode)
  (`KismetSystemLibrary.Delay` 2.0)
  (`self.K2_DestroyActor`))

(fn `GetAttachTransformRotation`
  (returns (`Attach Transform Up` :type "Transform Structure") (`Attach Transform Down` :type "Transform Structure") (`Attach Transform Right` :type "Transform Structure") (`Attach Transform Left` :type "Transform Structure"))
  (return (`SceneComponent.K2_GetComponentToWorld` (`self.AttachPointUp`)) (`SceneComponent.K2_GetComponentToWorld` (`self.AttachPointDown`)) (`SceneComponent.K2_GetComponentToWorld` (`self.AttachPointRight`)) (`SceneComponent.K2_GetComponentToWorld` (`self.AttachPointLeft`))))

(fn `UserConstructionScript`)