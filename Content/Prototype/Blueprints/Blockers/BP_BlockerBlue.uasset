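; BP_BlockerBlue is a prototype blue obstacle that gives way to a RunCharacter of matching color.
; Every Tick it reads the world color (WC) from PrototypeGameMode and switches the mesh between solid and alpha blue materials.
; When a RunCharacter overlaps the Trigger and its CharacterColor equals BlockingColor, the blocker destroys itself, though a note says it should disappear instead.
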(event `self.ReceiveTick`
  (params (DeltaSeconds :type "Float (single-precision)"))
  ;[1 1 1] Alpha
  ;;[1 1 1] Getting WC (world color) variable in GameMode (prototype)
  (bind _asprototype_game_mode (cast `/Game/Prototype/Blueprints/PrototypeGameMode` (`GameplayStatics.GetGameMode`)))
  (if (`|EnumEquality` (`/Game/Prototype/Blueprints/PrototypeGameMode.WC` _asprototype_game_mode) "NewEnumerator2")
    (`PrimitiveComponent.SetMaterial` (`self.StaticMeshBlue`) 0 "/Game/Prototype/Materials/AlphaMaterials/BlueMaterial_Alpha.BlueMaterial_Alpha")
    (else
      (`PrimitiveComponent.SetMaterial` (`self.StaticMeshBlue`) 0 "/Game/Prototype/Materials/BlueMaterial.BlueMaterial"))))

(event `self.Trigger.OnComponentBeginOverlap`
  (params (OverlappedComponent :type "PrimitiveComponent Object Reference") (OtherActor :type "Actor Object Reference") (OtherComp :type "PrimitiveComponent Object Reference") (OtherBodyIndex :type Integer) (bFromSweep :type Boolean) (SweepResult :type "HitResult Structure (by ref)"))
  (bind _asrun_character (cast `/Game/Prototype/Blueprints/RunCharacter` OtherActor))
  (if (`|EnumEquality` (`/Game/Prototype/Blueprints/RunCharacter.CharacterColor` _asrun_character) (`self.BlockingColor`))
    ;[1 1 1] Instead of destroying the obstacle actor, we have to make it dissapear
    (`self.K2_DestroyActor`)))

(fn `UserConstructionScript`
  (locals (RandomInt :type Integer)))