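; Color-coded blocker for the runner prototype, named as the green variant, that a RunCharacter clears by matching its color.
; Overlapping Trigger destroys the blocker when the character's CharacterColor equals BlockingColor.
; A separate ChangeColorTrigger volume sets the character's CanChangeColor on entry and clears it on exit, limiting color switching to that zone.
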(event `self.Trigger.OnComponentBeginOverlap`
  (params (OverlappedComponent :type "PrimitiveComponent Object Reference") (OtherActor :type "Actor Object Reference") (OtherComp :type "PrimitiveComponent Object Reference") (OtherBodyIndex :type Integer) (bFromSweep :type Boolean) (SweepResult :type "HitResult Structure (by ref)"))
  (bind _asrun_character (cast `/Game/Prototype/Blueprints/RunCharacter` OtherActor))
  (if (`|EnumEquality` (`/Game/Prototype/Blueprints/RunCharacter.CharacterColor` _asrun_character) (`self.BlockingColor`))
    (`self.K2_DestroyActor`)))

(event `self.ChangeColorTrigger.OnComponentBeginOverlap`
  (params (OverlappedComponent :type "PrimitiveComponent Object Reference") (OtherActor :type "Actor Object Reference") (OtherComp :type "PrimitiveComponent Object Reference") (OtherBodyIndex :type Integer) (bFromSweep :type Boolean) (SweepResult :type "HitResult Structure (by ref)"))
  (bind _asrun_character (cast `/Game/Prototype/Blueprints/RunCharacter` OtherActor))
  (set `/Game/Prototype/Blueprints/RunCharacter.CanChangeColor` true _asrun_character))

(event `self.ChangeColorTrigger.OnComponentEndOverlap`
  (params (OverlappedComponent :type "PrimitiveComponent Object Reference") (OtherActor :type "Actor Object Reference") (OtherComp :type "PrimitiveComponent Object Reference") (OtherBodyIndex :type Integer))
  (bind _asrun_character (cast `/Game/Prototype/Blueprints/RunCharacter` OtherActor))
  (set `/Game/Prototype/Blueprints/RunCharacter.CanChangeColor` false _asrun_character))

(fn `UserConstructionScript`
  (locals (RandomInt :type Integer)))