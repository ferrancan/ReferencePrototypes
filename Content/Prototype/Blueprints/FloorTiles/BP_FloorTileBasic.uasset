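; BP_FloorTileBasic is a prototype floor tile that spawns obstacles at four spots along its length, labelled 0m, 250m, 500m and 750m.
; Spawn Obstacles casts each spot's spawner reference to BP_BlockerSpawner and calls Spawn Blocker with the matching distance-named input.
; The calls run in sequence, so one failed cast skips the remaining spawners.
; The construction script is empty.
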(fn `Spawn Obstacles`
  (bind _asbp_blocker_spawner (cast `/Game/Prototype/Blueprints/Blockers/BP_BlockerSpawner` (`self.Spawner_0m`)))
  (`/Game/Prototype/Blueprints/Blockers/BP_BlockerSpawner.SpawnBlocker` _asbp_blocker_spawner (`self.0m`))
  (bind _asbp_blocker_spawner_2 (cast `/Game/Prototype/Blueprints/Blockers/BP_BlockerSpawner` (`self.Spawner_250m`)))
  (`/Game/Prototype/Blueprints/Blockers/BP_BlockerSpawner.SpawnBlocker` _asbp_blocker_spawner_2 (`self.250m`))
  (bind _asbp_blocker_spawner_3 (cast `/Game/Prototype/Blueprints/Blockers/BP_BlockerSpawner` (`self.Spawner_500m`)))
  (`/Game/Prototype/Blueprints/Blockers/BP_BlockerSpawner.SpawnBlocker` _asbp_blocker_spawner_3 (`self.500m`))
  (bind _asbp_blocker_spawner_4 (cast `/Game/Prototype/Blueprints/Blockers/BP_BlockerSpawner` (`self.Spawner_750m`)))
  (`/Game/Prototype/Blueprints/Blockers/BP_BlockerSpawner.SpawnBlocker` _asbp_blocker_spawner_4 (`self.750m`)))

(fn `UserConstructionScript`)