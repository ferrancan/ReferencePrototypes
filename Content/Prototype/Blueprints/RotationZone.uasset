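; RotationZone is a trigger zone that lets the RunCharacter rotate at a set spot in the level.
; Entering ActionTurnTrigger sets the character's OnlyTurnOnce flag and plays an enter sound at the trigger's location.
; Entering DoTurnTrigger stops the character's movement immediately and enables CanRotate for a brief delayed window before switching it off again.
; Both overlaps ignore other actors, and the turn itself is left to the character.
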(event `self.actionTurnTrigger.OnComponentBeginOverlap`
  (params (OverlappedComponent :type "PrimitiveComponent Object Reference") (OtherActor :type "Actor Object Reference") (OtherComp :type "PrimitiveComponent Object Reference") (OtherBodyIndex :type Integer) (bFromSweep :type Boolean) (SweepResult :type "HitResult Structure (by ref)"))
  (bind _asrun_character (cast `/Game/Prototype/Blueprints/RunCharacter` OtherActor))
  (set `/Game/Prototype/Blueprints/RunCharacter.onlyTurnOnce` true _asrun_character)
  (`GameplayStatics.SpawnSoundAtLocation` "/Game/Prototype/Sounds/RotationZone_Enter.RotationZone_Enter" (`SceneComponent.K2_GetComponentLocation` (`self.actionTurnTrigger`)) (struct) 1.0 1.0 0.0 null null))

(event `self.doTurnTrigger.OnComponentBeginOverlap`
  (params (OverlappedComponent :type "PrimitiveComponent Object Reference") (OtherActor :type "Actor Object Reference") (OtherComp :type "PrimitiveComponent Object Reference") (OtherBodyIndex :type Integer) (bFromSweep :type Boolean) (SweepResult :type "HitResult Structure (by ref)"))
  (bind _asrun_character (cast `/Game/Prototype/Blueprints/RunCharacter` OtherActor))
  (`MovementComponent.StopMovementImmediately` (`Character.CharacterMovement` _asrun_character))
  (set `/Game/Prototype/Blueprints/RunCharacter.canRotate` true _asrun_character)
  (`KismetSystemLibrary.Delay` 0.5)
  (set `/Game/Prototype/Blueprints/RunCharacter.canRotate` false _asrun_character))

(fn `UserConstructionScript`)